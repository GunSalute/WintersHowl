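; Eagle actor that watches for sheep and the player using an angle-based vision cone.
; On BeginPlay it stores its start location and caches every Sheep_BP actor plus the player character.
; Each tick it compares the direction to each cached actor against its forward vector, storing any within the cone as SeenActor.
; The check ignores distance and occlusion, the last match wins, and nothing here acts on the result.
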(event EventBeginPlay
  ;[1 1 1] Set start location and get all actors in game (Sheep and player for now)
  (Variables|Default|SetStartLocation (Transformation|GetActorLocation))
  (bind _outactors (Actor|GetAllActorsOfClass "/Game/BP/Sheep_BP.Sheep_BP_C"))
  (Variables|Default|SetAllActorsInGame _outactors)
  (Utilities|Array|Add (Variables|Default|GetAllActorsInGame) (Game|GetPlayerCharacter 0)))

(event EventTick
  (params (DeltaSeconds :type Float%20%28single-precision%29))
  (for _array_element (Variables|Default|GetAllActorsInGame)
    ;[1 1 1] If within vision cone - it's seen
    (if (< (Class|KismetMathLibrary|DegAcos (Math|Vector|DotProduct (Math|Vector|Normalize (- (Transformation|GetActorLocation _array_element) (Transformation|GetActorLocation))) (Transformation|GetActorForwardVector))) 6e+01)
      (Variables|Default|SetSeenActor _array_element))))

(fn ConstructionScript)